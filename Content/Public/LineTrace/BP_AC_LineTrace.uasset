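; BP_AC_LineTrace turns line trace hits into hover and press interaction for AC_Key actors and selection for BP_WidgetActor actors.
; It binds to hit detection on BeginPlay and tracks the hit actor, moving key hover from the previous actor to the new one.
; onTrigger presses or releases the hovered key, or toggles widget selection.
; While a key is held, hover changes are locked so release reaches the same key.
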(event Custom|FindActor
  (params (HitActor :type Actor%20Object%20Reference))
  (CallFunction|HoverSetting HitActor))

(event Custom|HoverSetting
  (params (NewHover :type Actor%20Object%20Reference))
  ;[0.15 0.15 0.15 0.5] Hover Event
  (bind _output_get (Variables|Default|SetHoverNextActor NewHover))
  (if (!= _output_get (Variables|Default|GetHoverCurrentActor))
    (if (not (Variables|Default|GetbTrigging))
      (Utilities|FlowControl|Sequence
        (:then_0
          (bind _asac_key (Utilities|Casting|CastToAC_Key (Variables|Default|GetHoverCurrentActor)))
          (Class|ACKey|SetHover _asac_key false))
        (:then_1
          (Variables|Default|SetHoverCurrentActor _output_get))
        (:then_2
          (bind _asac_key_2 (Utilities|Casting|CastToAC_Key (Variables|Default|GetHoverCurrentActor)))
          (Class|ACKey|SetHover _asac_key_2 true))))))

(event Custom|onTrigger
  (params (Condition :type Boolean))
  (bind _hovercurrentactor (Variables|Default|GetHoverCurrentActor))
  ;[0.15 0.15 0.15 0.5] Trigger Event
  (if Condition
    (Utilities|FlowControl|Sequence
      (:then_0
        (bind _asac_key (Utilities|Casting|CastToAC_Key _hovercurrentactor))
        (Class|ACKey|KeyPress _asac_key)
        (Variables|Default|SetbTrigging true))
      (:then_1
        (bind _asbp_widget_actor (Utilities|Casting|CastToBP_WidgetActor _hovercurrentactor))
        (Default|Seleced _asbp_widget_actor true)))
    (else
      (Utilities|FlowControl|Sequence
        (:then_0
          (bind _asac_key_2 (Utilities|Casting|CastToAC_Key _hovercurrentactor))
          (Class|ACKey|KeyRelease _asac_key_2 false)
          (Variables|Default|SetbTrigging false))
        (:then_1
          (bind _asbp_widget_actor_2 (Utilities|Casting|CastToBP_WidgetActor _hovercurrentactor))
          (Default|Seleced _asbp_widget_actor_2 false))))))

(event EventBeginPlay
  ;[0.15 0.15 0.15 0.5] Bind Actor Changed
  (EventDispatchers|BindEventtoOnHitDetected (EventDispatchers|CreateEvent :!event Custom|FindActor)))

(event EventTick
  (params (DeltaSeconds :type Float%20%28single-precision%29)))