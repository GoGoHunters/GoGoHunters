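; Museum exhibition stand actor that hosts three BP_MuseumPlaceArea child actors as grid placement areas.
; The construction script pushes the stand's grid counts, cell size, uniform scale and debug display into all three areas, so they share one configuration.
; Each setter casts the child actors in sequence and stops at the first failed cast; the stand has no active runtime logic.
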(event EventBeginPlay)

(event Collision|EventActorBeginOverlap
  (params (OtherActor :type Actor%20Object%20Reference)))

(event EventTick
  (params (DeltaSeconds :type Float%20%28single-precision%29)))

(fn ConstructionScript
  (CallFunction|SetShowGridDebug (Variables|Default|GetbDebug))
  (CallFunction|SetGridX (Variables|Default|GetGridX))
  (CallFunction|SetGridY (Variables|Default|GetGridY))
  (CallFunction|SetCellSize (Variables|Default|GetCellSize))
  (CallFunction|SetScale (Variables|Default|GetScale)))

(fn SetGridX
  (params (NewGridX :type Integer))
  (bind _asbp_museum_place_area (Utilities|Casting|CastToBP_MuseumPlaceArea (Variables|/Script/Engine.ChildActorComponent|GetChildActor (Variables|Default|GetBP_MuseumPlaceArea))))
  (bind _output_get (Variables|/Script/GoGoHunters.CMuseumPlaceArea|SetGridXCount _asbp_museum_place_area NewGridX))
  (bind _asbp_museum_place_area_2 (Utilities|Casting|CastToBP_MuseumPlaceArea (Variables|/Script/Engine.ChildActorComponent|GetChildActor (Variables|Default|GetBP_MuseumPlaceArea1))))
  (bind _output_get_2 (Variables|/Script/GoGoHunters.CMuseumPlaceArea|SetGridXCount _asbp_museum_place_area_2 _output_get))
  (bind _asbp_museum_place_area_3 (Utilities|Casting|CastToBP_MuseumPlaceArea (Variables|/Script/Engine.ChildActorComponent|GetChildActor (Variables|Default|GetBP_MuseumPlaceArea2))))
  (Variables|/Script/GoGoHunters.CMuseumPlaceArea|SetGridXCount _asbp_museum_place_area_3 _output_get_2))

(fn SetGridY
  (params (NewY :type Integer))
  (bind _asbp_museum_place_area (Utilities|Casting|CastToBP_MuseumPlaceArea (Variables|/Script/Engine.ChildActorComponent|GetChildActor (Variables|Default|GetBP_MuseumPlaceArea))))
  (bind _output_get (Variables|/Script/GoGoHunters.CMuseumPlaceArea|SetGridYCount _asbp_museum_place_area NewY))
  (bind _asbp_museum_place_area_2 (Utilities|Casting|CastToBP_MuseumPlaceArea (Variables|/Script/Engine.ChildActorComponent|GetChildActor (Variables|Default|GetBP_MuseumPlaceArea1))))
  (bind _output_get_2 (Variables|/Script/GoGoHunters.CMuseumPlaceArea|SetGridYCount _asbp_museum_place_area_2 _output_get))
  (bind _asbp_museum_place_area_3 (Utilities|Casting|CastToBP_MuseumPlaceArea (Variables|/Script/Engine.ChildActorComponent|GetChildActor (Variables|Default|GetBP_MuseumPlaceArea2))))
  (Variables|/Script/GoGoHunters.CMuseumPlaceArea|SetGridYCount _asbp_museum_place_area_3 _output_get_2))

(fn SetCellSize
  (params (NewCellSize :type Float%20%28double-precision%29))
  (bind _asbp_museum_place_area (Utilities|Casting|CastToBP_MuseumPlaceArea (Variables|/Script/Engine.ChildActorComponent|GetChildActor (Variables|Default|GetBP_MuseumPlaceArea))))
  (bind _output_get (Variables|/Script/GoGoHunters.CMuseumPlaceArea|SetCellSize _asbp_museum_place_area NewCellSize))
  (bind _asbp_museum_place_area_2 (Utilities|Casting|CastToBP_MuseumPlaceArea (Variables|/Script/Engine.ChildActorComponent|GetChildActor (Variables|Default|GetBP_MuseumPlaceArea1))))
  (bind _output_get_2 (Variables|/Script/GoGoHunters.CMuseumPlaceArea|SetCellSize _asbp_museum_place_area_2 _output_get))
  (bind _asbp_museum_place_area_3 (Utilities|Casting|CastToBP_MuseumPlaceArea (Variables|/Script/Engine.ChildActorComponent|GetChildActor (Variables|Default|GetBP_MuseumPlaceArea2))))
  (Variables|/Script/GoGoHunters.CMuseumPlaceArea|SetCellSize _asbp_museum_place_area_3 _output_get_2))

(fn SetShowGridDebug
  (params (NewDebug :type Boolean))
  (bind _asbp_museum_place_area (Utilities|Casting|CastToBP_MuseumPlaceArea (Variables|/Script/Engine.ChildActorComponent|GetChildActor (Variables|Default|GetBP_MuseumPlaceArea))))
  (bind _output_get (Variables|/Script/GoGoHunters.CMuseumPlaceArea|SetbShowGridDebug _asbp_museum_place_area NewDebug))
  (bind _asbp_museum_place_area_2 (Utilities|Casting|CastToBP_MuseumPlaceArea (Variables|/Script/Engine.ChildActorComponent|GetChildActor (Variables|Default|GetBP_MuseumPlaceArea1))))
  (bind _output_get_2 (Variables|/Script/GoGoHunters.CMuseumPlaceArea|SetbShowGridDebug _asbp_museum_place_area_2 _output_get))
  (bind _asbp_museum_place_area_3 (Utilities|Casting|CastToBP_MuseumPlaceArea (Variables|/Script/Engine.ChildActorComponent|GetChildActor (Variables|Default|GetBP_MuseumPlaceArea2))))
  (Variables|/Script/GoGoHunters.CMuseumPlaceArea|SetbShowGridDebug _asbp_museum_place_area_3 _output_get_2))

(fn SetScale
  (params (NewScale :type Vector))
  (bind _asbp_museum_place_area (Utilities|Casting|CastToBP_MuseumPlaceArea (Variables|/Script/Engine.ChildActorComponent|GetChildActor (Variables|Default|GetBP_MuseumPlaceArea))))
  (bind _output_get (Variables|/Script/GoGoHunters.CMuseumPlaceArea|SetCellUniformScale _asbp_museum_place_area NewScale))
  (bind _asbp_museum_place_area_2 (Utilities|Casting|CastToBP_MuseumPlaceArea (Variables|/Script/Engine.ChildActorComponent|GetChildActor (Variables|Default|GetBP_MuseumPlaceArea1))))
  (bind _output_get_2 (Variables|/Script/GoGoHunters.CMuseumPlaceArea|SetCellUniformScale _asbp_museum_place_area_2 _output_get))
  (bind _asbp_museum_place_area_3 (Utilities|Casting|CastToBP_MuseumPlaceArea (Variables|/Script/Engine.ChildActorComponent|GetChildActor (Variables|Default|GetBP_MuseumPlaceArea2))))
  (Variables|/Script/GoGoHunters.CMuseumPlaceArea|SetCellUniformScale _asbp_museum_place_area_3 _output_get_2))