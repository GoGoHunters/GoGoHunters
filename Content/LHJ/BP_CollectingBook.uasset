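; Collecting book actor that animates itself in and out when ActiveAnim is called with an Active flag.
; On activation, a timeline drives uniform actor scale, and a valid CollectingBook reference gets its data initialized, after which the player distance check flag is set and collision is enabled.
; On deactivation, the timeline reverses from its end and collision is disabled.
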(event EventBeginPlay)

(event Collision|EventActorBeginOverlap
  (params (OtherActor :type Actor%20Object%20Reference)))

(event EventTick
  (params (DeltaSeconds :type Float%20%28single-precision%29)))

(event EventActiveAnim
  (params (bActive :type Boolean))
  (if bActive
    (Utilities|FlowControl|Sequence
      (:then_0
        (bind _alpha (Timeline|Timeline Play)
          (:Update
            (Transformation|SetActorScale3D (Math|Conversions|ToVector(Float) _alpha)))))
      (:then_1
        (bind _collectingbook (Variables|Default|GetCollectingBook)
          (:then
            (Class|CCollectingBookWidget|InitData _collectingbook)
            (Variables|Default|SetbStartPlayerDistCheck true)
            (Collision|SetActorEnableCollision true))
          (:else))))
    (else
      (Utilities|FlowControl|Sequence
        (:then_0
          (Timeline|Timeline ReverseFromEnd))
        (:then_1
          (Collision|SetActorEnableCollision false))))))

(fn ConstructionScript)