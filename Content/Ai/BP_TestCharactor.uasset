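; BP_TestCharactor is a test actor that toggles recording on an AI actor with the H key.
; On BeginPlay it enables input from the first player controller.
; Pressing H finds all BP_P_AI actors and calls ActivateRecord(true) on the first one, while releasing calls it with false, making it push-to-record.
; If no valid actor is found, it prints a placeholder "Hello" string.
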(event EventBeginPlay
  (Input|EnableInput (Game|GetPlayerController 0)))

(event Collision|EventActorBeginOverlap
  (params (OtherActor :type Actor%20Object%20Reference)))

(event EventTick
  (params (DeltaSeconds :type Float%20%28single-precision%29)))

(event Input|KeyboardEvents|H
  (params (Key :type Key%20Structure :default "None"))
  (:Pressed
    (bind _outactors (Actor|GetAllActorsOfClass "/Game/Ai/Logic/BP_P_AI.BP_P_AI_C"))
    (Utilities|IsValid (Utilities|Array|Get(acopy) _outactors)
      (:Is%20Valid
        (Default|ActivateRecord (Utilities|Array|Get(acopy) _outactors) true))
      (:Is%20Not%20Valid
        (Development|PrintString "Hello"))))
  (:Released
    (bind _outactors_2 (Actor|GetAllActorsOfClass "/Game/Ai/Logic/BP_P_AI.BP_P_AI_C"))
    (Utilities|IsValid (Utilities|Array|Get(acopy) _outactors_2)
      (:Is%20Valid
        (Default|ActivateRecord (Utilities|Array|Get(acopy) _outactors_2) false))
      (:Is%20Not%20Valid
        (Development|PrintString "Hello")))))

(fn ConstructionScript)