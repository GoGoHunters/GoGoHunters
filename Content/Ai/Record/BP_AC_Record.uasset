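; BP_AC_Record is an AI recording component that relays microphone audio and files over a WebSocket.
; On BeginPlay it binds an event to microphone-capture notifications.
; Its audio and file events send captured bytes or a file path's contents through the WebSocket held by BP_GI_Base, the game instance.
; RecordActivate stores a recording-ready flag, which none of the send events here check.
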(event Custom|MicroPthoneData
  (params (CapturedAudioBytes :type Array%20of%20Bytes))
  (bind _asbp_gi_base (Utilities|Casting|CastToBP_GI_Base (Game|GetGameInstance)))
  (Class|UWebSocketManager|WebSocketSendByteData (Variables|/Game/Ai/WebSocket/BP_GI_Base.BP_GI_Base_C|GetWebSocket _asbp_gi_base) CapturedAudioBytes))

(event Custom|File%20Send
  (params (FilePath :type String))
  (bind _asbp_gi_base (Utilities|Casting|CastToBP_GI_Base (Game|GetGameInstance)))
  (Class|UWebSocketManager|WebSocketSendByteFile (Variables|/Game/Ai/WebSocket/BP_GI_Base.BP_GI_Base_C|GetWebSocket _asbp_gi_base) FilePath))

(event Custom|RecordActivate
  (params (Is%20Ready%20to%20Recording :type Boolean))
  (Variables|Default|SetisReadyToRecording Is%20Ready%20to%20Recording))

(event EventBeginPlay
  (Utilities|FlowControl|Sequence
    (:then_0
      (EventDispatchers|BindEventtoOnMicrophoneDataCaptured (EventDispatchers|CreateEvent :!event Custom|MicroPthoneData)))))