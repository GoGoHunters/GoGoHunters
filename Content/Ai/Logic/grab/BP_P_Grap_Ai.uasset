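; BP_P_Grap_Ai is an AI-controlled floating pawn that can be grabbed and plays audio received over a WebSocket.
; On BeginPlay it sets its movement tuning and binds to the byte-data event of the WebSocket held by BP_GI_Base.
; Received bytes are meant to play through BPACAudio.
; Grab and Release write the bIsGrap flag and GrapOwner to the AI controller's Blackboard, setting or clearing the owner.
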(event Custom|CustomEvent
  (params (ReceivedBytes :type Array%20of%20Bytes))
  (Class|ACAudio|PlayAudiofromBytes (Variables|Default|GetBP_AC_Audio) ReceivedBytes))

(event Custom|Grab
  (params (OwnPawn :type Pawn%20Object%20Reference))
  (bind _self self)
  (bind _returnvalue (AI|GetAIController _self))
  (bind _returnvalue_2 (AI|GetBlackboard _returnvalue))
  (AI|Components|Blackboard|SetValueasBool _returnvalue_2 (Utilities|Name|MakeLiteralName "bIsGrap") true)
  (AI|Components|Blackboard|SetValueasObject _returnvalue_2 (Utilities|Name|MakeLiteralName "GrapOwner") OwnPawn))

(event Custom|Release
  (params (OwnPawn :type Pawn%20Object%20Reference))
  (bind _self self)
  (bind _returnvalue (AI|GetAIController _self))
  (bind _returnvalue_2 (AI|GetBlackboard _returnvalue))
  (AI|Components|Blackboard|SetValueasBool _returnvalue_2 (Utilities|Name|MakeLiteralName "bIsGrap") false)
  (AI|Components|Blackboard|SetValueasObject _returnvalue_2 (Utilities|Name|MakeLiteralName "GrapOwner") 0))

(event EventBeginPlay
  (bind _floatingpawnmovement (Variables|Default|GetFloatingPawnMovement))
  (Utilities|FlowControl|Sequence
    (:then_0
      (Variables|/Script/Engine.FloatingPawnMovement|SetMaxSpeed _floatingpawnmovement 3e+02)
      (Variables|/Script/Engine.FloatingPawnMovement|SetAcceleration _floatingpawnmovement 1e+02)
      (Variables|/Script/Engine.FloatingPawnMovement|SetDeceleration _floatingpawnmovement 1e+02))
    (:then_1
      (bind _asbp_gi_base (Utilities|Casting|CastToBP_GI_Base (Game|GetGameInstance)))
      (EventDispatchers|BindEventtoOnByteDataReceived (Variables|/Game/Ai/WebSocket/BP_GI_Base.BP_GI_Base_C|GetWebSocket _asbp_gi_base) (EventDispatchers|CreateEvent :!event Custom|CustomEvent)))))

(fn ConstructionScript)