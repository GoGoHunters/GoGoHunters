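; BP_P_Following is an AI pawn that feeds player detection and talking state to its Blackboard, likely for following behavior.
; On BeginPlay it configures slow FloatingPawnMovement.
; PawnSensing sets bFindPlayer by whether the seen pawn is the player, then sets bTalking after a delay, whichever pawn was seen.
; The player leaving the Sphere overlap clears both keys, without cancelling a pending delay.
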(event OnSeePawn(PawnSensing)
  (params (Pawn :type Pawn%20Object%20Reference))
  (bind _self self)
  (bind _returnvalue (AI|GetAIController _self))
  (bind _returnvalue_2 (AI|GetBlackboard _returnvalue))
  (AI|Components|Blackboard|SetValueasBool _returnvalue_2 (Utilities|Name|MakeLiteralName "bFindPlayer") (== Pawn (Game|Player|GetPlayerPawn 0)))
  ;[0.15 0 0 0.5] delay 에러 사항 참고
  (Utilities|FlowControl|Delay 3.0)
  (AI|Components|Blackboard|SetValueasBool _returnvalue_2 (Utilities|Name|MakeLiteralName "bTalking") true))

(event OnComponentEndOverlap(Sphere)
  (params (OverlappedComponent :type Primitive%20Component%20Object%20Reference) (OtherActor :type Actor%20Object%20Reference) (OtherComp :type Primitive%20Component%20Object%20Reference) (OtherBodyIndex :type Integer))
  (bind _self self)
  (bind _returnvalue (AI|GetAIController _self))
  (bind _returnvalue_2 (AI|GetBlackboard _returnvalue))
  (if (== OtherActor (Game|Player|GetPlayerPawn 0))
    (AI|Components|Blackboard|SetValueasBool _returnvalue_2 (Utilities|Name|MakeLiteralName "bFindPlayer") false)
    (AI|Components|Blackboard|SetValueasBool _returnvalue_2 (Utilities|Name|MakeLiteralName "bTalking") false)))

(event EventBeginPlay
  (bind _floatingpawnmovement (Variables|Default|GetFloatingPawnMovement))
  (Variables|/Script/Engine.FloatingPawnMovement|SetMaxSpeed _floatingpawnmovement 3e+02)
  (Variables|/Script/Engine.FloatingPawnMovement|SetAcceleration _floatingpawnmovement 1e+02)
  (Variables|/Script/Engine.FloatingPawnMovement|SetDeceleration _floatingpawnmovement 1e+02))

(event Collision|EventActorBeginOverlap
  (params (OtherActor :type Actor%20Object%20Reference)))

(event EventTick
  (params (DeltaSeconds :type Float%20%28single-precision%29)))

(fn ConstructionScript)