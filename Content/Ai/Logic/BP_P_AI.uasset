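; Pawn for Tami, the VR player's AI companion, which hovers near the shoulder or moves to a target while facing the camera.
; Recording and WebSocket byte audio drive voice exchanges, updating anim flags, mesh and Blackboard as Tami thinks or talks.
; Tutorial steps show a widget, animation and sound, ending on a timer or skip via BP_TutorialManager.
; Excavation-level events play phase narration, some chained by delays.
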(event OnAudioPlaybackEnded(BP_AC_Audio)
  ;[0.15 0.15 0.15 0.5] Audio Play
  (Development|PrintString "Audio play Finish")
  (CallFunction|SetTamiMesh "NewEnumerator3")
  (CallFunction|LookReset)
  (Variables|/Script/GoGoHunters.AC_Record|SetisWaitForServer (Variables|Default|GetBP_AC_Record) false)
  ;;[0.6628 0.5912 0 0.5] AnimBlueprint
  (Variables|/Game/Ai/Model/Tami/ABP_Tami.ABP_Tami_C|SetbIsTalk (Variables|Default|GetAs%20ABP%20Tami) false)
  ;[0.5977 0.1004 0.1004 0.5] BlackBoard
  (AI|Components|Blackboard|SetValueasBool (AI|GetBlackboard (AI|GetAIController self)) (Utilities|Name|MakeLiteralName "bTalking") false))

(event OnRecordingStateChanged(BP_AC_Record)
  (params (bIsRecording :type Boolean))
  ;[0.15 0.15 0.15 0.5] Think
  (CallFunction|BeThink bIsRecording))

(event OnComponentBeginOverlap(Sphere)
  (params (OverlappedComponent :type Primitive%20Component%20Object%20Reference) (OtherActor :type Actor%20Object%20Reference) (OtherComp :type Primitive%20Component%20Object%20Reference) (OtherBodyIndex :type Integer) (bFromSweep :type Boolean) (SweepResult :type Hit%20Result%20Structure%20%28by%20ref%29)))

(event Custom|PlayAudio
  (params (ReceivedBytes :type Array%20of%20Bytes))
  ;[0.15 0.15 0.15 0.5] Audio Play
  (CallFunction|SetTamiMesh "NewEnumerator1")
  (bind _asbp_mh_vrplayer (Utilities|Casting|CastToBP_MH_VRPlayer (Game|Player|GetPlayerPawn 0))
    (:then
      (CallFunction|Lookat _asbp_mh_vrplayer))
    (:CastFailed
      _))
  ;;[0.6628 0.5912 0 0.5] AnimBlueprint
  (Variables|/Game/Ai/Model/Tami/ABP_Tami.ABP_Tami_C|SetbIsTalk (Variables|Default|GetAs%20ABP%20Tami) true)
  ;[0.5977 0.1004 0.1004 0.5] BlackBoard
  (AI|Components|Blackboard|SetValueasBool (AI|GetBlackboard (AI|GetAIController self)) (Utilities|Name|MakeLiteralName "bTalking") true)
  (Class|ACAudio|PlayAudiofromBytes (Variables|Default|GetBP_AC_Audio) ReceivedBytes))

(event Custom|Grab
  (params (bisGrap :type Boolean) (GrabOwner :type Pawn%20Object%20Reference))
  (bind _self self)
  (bind _returnvalue (AI|GetAIController _self))
  (bind _returnvalue_2 (AI|GetBlackboard _returnvalue))
  (bind _output_get (Variables|Default|SetbisGrap bisGrap))
  (AI|Components|Blackboard|SetValueasBool _returnvalue_2 (Utilities|Name|MakeLiteralName "bIsGrap") _output_get)
  (AI|Components|Blackboard|SetValueasObject _returnvalue_2 (Utilities|Name|MakeLiteralName "GrapOwner") GrabOwner))

(event Custom|CallBack_Tutorial
  ;[0.15 0.15 0.15 0.5] 튜토리얼 함수
  (bind _tutorialmanager (Variables|Default|GetTutorialManager)
    (:then
      (Class|CTutorialManager|StopTutorial _tutorialmanager))
    (:else
      _))
  (bind _tutorialwidget (Variables|Default|GetTutorialWidget)
    (:then
      (Class|CTutorialUI|EndTutorial _tutorialwidget)
      (CallFunction|SetWidgetVisible false))
    (:else)))

(event Custom|CustomEvent
  ;[0.15 0.15 0.15 0.5] Audio receive
  (Variables|/Script/GoGoHunters.AC_Record|SetisWaitForServer (Variables|Default|GetBP_AC_Record) true))

(event Custom|SkipTutorial
  ;[0.15 0.15 0.15 0.5] 튜토리얼 함수
  (CallFunction|CallBackTutorial)
  (Utilities|Time|ClearandInvalidateTimerbyHandle (Variables|Default|GetTutorialCallBackHandle)))

(event Custom|SetWidgetVisible
  (params (IsVisible :type Boolean))
  (bind _widget (Variables|Default|GetWidget))
  ;[0.15 0.15 0.15 0.5] 튜토리얼 함수
  (Rendering|SetVisibility _widget IsVisible false)
  (if IsVisible
    (Collision|SetCollisionEnabled _widget "QueryOnly")
    (else
      (Collision|SetCollisionEnabled _widget "NoCollision"))))

(event Custom|PlayExcavationStart
  (bind _tutorialmanager (Variables|Default|GetTutorialManager))
  ;[0.15 0.15 0.15 0.5] 발굴 레벨에서 재생할 타미 대사
  (Audio|PlaySoundatLocation "/Game/LHJ/Tutorial/Files/Sounds/Excavation/SW_Start1.SW_Start1" (Transformation|GetActorLocation) "0, 0, 0" 1.0 1.0 0.0 0 0 0 0)
  (Utilities|FlowControl|Delay 13.0)
  (Utilities|IsValid _tutorialmanager
    (:Is%20Valid
      (Class|CTutorialManager|StartTutorial _tutorialmanager "SelectDetector"))))

(event Custom|PlayExcavationPhase1_DetectorPercent100
  ;[0.15 0.15 0.15 0.5] 발굴 레벨에서 재생할 타미 대사
  (Audio|PlaySoundatLocation "/Game/LHJ/Tutorial/Files/Sounds/Excavation/SW_Phase1_5_DetectorPercent100.SW_Phase1_5_DetectorPercent100" (Transformation|GetActorLocation) "0, 0, 0" 1.0 1.0 0.0 0 0 0 0))

(event Custom|PlayExcavationPhase1_DetectorPercent
  ;[0.15 0.15 0.15 0.5] 발굴 레벨에서 재생할 타미 대사
  (Audio|PlaySoundatLocation "/Game/LHJ/Tutorial/Files/Sounds/Excavation/SW_Phase1_4_DetectorPercent.SW_Phase1_4_DetectorPercent" (Transformation|GetActorLocation) "0, 0, 0" 1.0 1.0 0.0 0 0 0 0))

(event Custom|PlayExcavationPhase4_DiscoveryRelic
  ;[0.15 0.15 0.15 0.5] 발굴 레벨에서 재생할 타미 대사
  (Audio|PlaySoundatLocation "/Game/LHJ/Tutorial/Files/Sounds/Excavation/SW_Phase5_2_DiscoveryRelic.SW_Phase5_2_DiscoveryRelic" (Transformation|GetActorLocation) "0, 0, 0" 1.0 1.0 0.0 0 0 0 0)
  (Utilities|FlowControl|Delay 2.5)
  (CallFunction|PlayExcavationPhase4StartBrush))

(event Custom|PlayExcavationPhase2_StartFlag
  ;[0.15 0.15 0.15 0.5] 발굴 레벨에서 재생할 타미 대사
  (Audio|PlaySoundatLocation "/Game/LHJ/Tutorial/Files/Sounds/Excavation/SW_Phase2_1_StartFlag_join.SW_Phase2_1_StartFlag_join" (Transformation|GetActorLocation) "0, 0, 0" 1.0 1.0 0.0 0 0 0 0))

(event Custom|LookAt
  (params (LookObject :type Actor%20Object%20Reference))
  ;[0.15 0.15 0.15 0.5] Look
  (Variables|Default|SetbisLooking true)
  (Variables|Default|SetLookObject LookObject))

(event Custom|PlayExcavationPhase2_PlantedFlag
  ;[0.15 0.15 0.15 0.5] 발굴 레벨에서 재생할 타미 대사
  (Audio|PlaySoundatLocation "/Game/LHJ/Tutorial/Files/Sounds/Excavation/SW_Phase2_4_PlantedFlag.SW_Phase2_4_PlantedFlag" (Transformation|GetActorLocation) "0, 0, 0" 1.0 1.0 0.0 0 0 0 0)
  (Utilities|FlowControl|Delay 4.0)
  (CallFunction|PlayExcavationPhase3StartShovel))

(event Custom|PlayExcavationPhase3_StartShovel
  ;[0.15 0.15 0.15 0.5] 발굴 레벨에서 재생할 타미 대사
  (Audio|PlaySoundatLocation "/Game/LHJ/Tutorial/Files/Sounds/Excavation/SW_Phase3_1_StartShovel_join.SW_Phase3_1_StartShovel_join" (Transformation|GetActorLocation) "0, 0, 0" 1.0 1.0 0.0 0 0 0 0))

(event Custom|PlayExcavationPhase3_VisibleRelic
  ;[0.15 0.15 0.15 0.5] 발굴 레벨에서 재생할 타미 대사
  (Audio|PlaySoundatLocation "/Game/LHJ/Tutorial/Files/Sounds/Excavation/SW_Phase3_5_VisibleRelic.SW_Phase3_5_VisibleRelic" (Transformation|GetActorLocation) "0, 0, 0" 1.0 1.0 0.0 0 0 0 0))

(event Custom|PlayExcavationPhase4_StartBrush
  ;[0.15 0.15 0.15 0.5] 발굴 레벨에서 재생할 타미 대사
  (Audio|PlaySoundatLocation "/Game/LHJ/Tutorial/Files/Sounds/Excavation/SW_Phase4_1_StartBrush_join.SW_Phase4_1_StartBrush_join" (Transformation|GetActorLocation) "0, 0, 0" 1.0 1.0 0.0 0 0 0 0))

(event Custom|PlayExcavationEnd
  ;[0.15 0.15 0.15 0.5] 발굴 레벨에서 재생할 타미 대사
  (Audio|PlaySoundatLocation "/Game/LHJ/Tutorial/Files/Sounds/Excavation/SW_End.SW_End" (Transformation|GetActorLocation) "0, 0, 0" 1.0 1.0 0.0 0 0 0 0))

(event Custom|LookReset
  ;[0.15 0.15 0.15 0.5] Look
  (Variables|Default|SetbisLooking false))

(event Custom|PlayExcavationPhase5_StartCollection
  ;[0.15 0.15 0.15 0.5] 발굴 레벨에서 재생할 타미 대사
  (Audio|PlaySoundatLocation "/Game/LHJ/Tutorial/Files/Sounds/Excavation/SW_Phase5_1_StartCollection_join.SW_Phase5_1_StartCollection_join" (Transformation|GetActorLocation) "0, 0, 0" 1.0 1.0 0.0 0 0 0 0))

(event Custom|PlayExcavationPhase5_ExplainUsingTweezers2
  ;[0.15 0.15 0.15 0.5] 발굴 레벨에서 재생할 타미 대사
  (Audio|PlaySoundatLocation "/Game/LHJ/Tutorial/Files/Sounds/Excavation/SW_Phase5_6_ExplainUsingTweezers2.SW_Phase5_6_ExplainUsingTweezers2" (Transformation|GetActorLocation) "0, 0, 0" 1.0 1.0 0.0 0 0 0 0))

(event Custom|PlayExcavationCompleted1
  ;[0.15 0.15 0.15 0.5] 발굴 레벨에서 재생할 타미 대사
  (Audio|PlaySoundatLocation "/Game/LHJ/Tutorial/Files/Sounds/Excavation/SW_CompletedExcavation1.SW_CompletedExcavation1" (Transformation|GetActorLocation) "0, 0, 0" 1.0 1.0 0.0 0 0 0 0))

(event Custom|PlayExcavationCompleted2
  ;[0.15 0.15 0.15 0.5] 발굴 레벨에서 재생할 타미 대사
  (Audio|PlaySoundatLocation "/Game/LHJ/Tutorial/Files/Sounds/Excavation/SW_CompletedExcavation2.SW_CompletedExcavation2" (Transformation|GetActorLocation) "0, 0, 0" 1.0 1.0 0.0 0 0 0 0)
  (Utilities|FlowControl|Delay 4.0)
  (CallFunction|PlayExcavationEnd))

(event Custom|PlayExcavationCompliment
  ;[0.15 0.15 0.15 0.5] 발굴 레벨에서 재생할 타미 대사
  (Audio|PlaySoundatLocation "/Game/LHJ/Tutorial/Files/Sounds/Excavation/SW_Compliment.SW_Compliment" (Transformation|GetActorLocation) "0, 0, 0" 1.0 1.0 0.0 0 0 0 0))

(event Custom|SetMoveTo
  (params (Target :type Vector))
  ;[0.15 0.15 0.15 0.5] Move To Location
  (Variables|Default|SetisMoveTo true)
  (Variables|Default|SetMoveToLocation Target))

(event Custom|UnsetMoveTo
  ;[0.15 0.15 0.15 0.5] Move To Location
  (Variables|Default|SetisMoveTo false)
  (Variables|Default|SetMoveToLocation "0, 0, 0"))

(event Custom|BeThink
  (params (isThink :type Boolean))
  ;[0.15 0.15 0.15 0.5] Think
  ;;[0.6628 0.5912 0 0.5] AnimBlueprint
  (Variables|/Game/Ai/Model/Tami/ABP_Tami.ABP_Tami_C|SetbIsThink (Variables|Default|GetAs%20ABP%20Tami) isThink))

(event Custom|Activate%20Record
  (params (Is%20Ready%20to%20Recording :type Boolean))
  ;[0.15 0.15 0.15 0.5] 외부 사용함수
  ;;[0.15 0.15 0.15 0.5] Record 활성화
  (Default|RecordActivate (Variables|Default|GetBP_AC_Record) Is%20Ready%20to%20Recording))

(event Custom|StartTutorial
  (params (TutorialData :type C%20Tutorial%20Data%20Structure))
  (bind (_stepid _tutorialimage _tutorialanimation _tutorialsound) (Utilities|Struct|BreakCTutorialData TutorialData))
  ;[0.15 0.15 0.15 0.5] 튜토리얼 함수
  (CallFunction|SetWidgetVisible true)
  (|CollapseGraph TutorialData _tutorialanimation _tutorialsound
    (:Is%20Not%20Valid
      (Variables|Default|SetDuration 5.0))
    (:then
      (Variables|Default|SetDuration (Variables|/Script/Engine.SoundBase|GetDuration _tutorialsound))))
  (bind _returnvalue (Utilities|Time|SetTimerbyEvent (delegate Custom|CallBack_Tutorial) (Variables|Default|GetDuration)))
  (Variables|Default|SetTutorialCallBackHandle _returnvalue))

(event Custom|DoHappy
  ;[0.15 0.15 0.15 0.5] Happy
  ;[0.6628 0.5912 0 0.5] AnimBlueprint
  (Variables|/Game/Ai/Model/Tami/ABP_Tami.ABP_Tami_C|SetbIsHappy (Variables|Default|GetAs%20ABP%20Tami) false))

(event EventBeginPlay
  (bind _floatingpawnmovement (Variables|Default|GetFloatingPawnMovement))
  (Utilities|FlowControl|Sequence
    (:then_0
      (Variables|/Script/Engine.FloatingPawnMovement|SetMaxSpeed _floatingpawnmovement 3e+02)
      (Variables|/Script/Engine.FloatingPawnMovement|SetAcceleration _floatingpawnmovement 256.0)
      (Variables|/Script/Engine.FloatingPawnMovement|SetDeceleration _floatingpawnmovement 256.0))
    (:then_1
      (bind _asabp_tami (Utilities|Casting|CastToABP_Tami (Components|SkeletalMesh|GetAnimInstance (Variables|Default|GetSkeletalMesh)))
        (:then
          (Variables|Default|SetAs%20ABP%20Tami _asabp_tami))
        (:CastFailed
          (Development|PrintText "Cast Error ABP_Tami"))))
    (:then_2
      (EventDispatchers|BindEventtoOnRecordingEnded (Variables|Default|GetBP_AC_Record) (EventDispatchers|CreateEvent :!event Custom|CustomEvent)))
    (:then_3
      (bind _asbp_gi_base (Utilities|Casting|CastToBP_GI_Base (Game|GetGameInstance)))
      (EventDispatchers|BindEventtoOnByteDataReceived (Variables|/Game/Ai/WebSocket/BP_GI_Base.BP_GI_Base_C|GetWebSocket _asbp_gi_base) (EventDispatchers|CreateEvent :!event Custom|PlayAudio)))
    (:then_4
      (Variables|Default|SetPlayerPawn (Game|Player|GetPlayerPawn 0))
      ;[0.15 0.15 0.15 0.5] 튜토리얼 추가 노드
      (bind _aswbp_tutorial (Utilities|Casting|CastToWBP_Tutorial (UserInterface|GetWidget (Variables|Default|GetWidget))))
      (bind _output_get (Variables|Default|SetTutorialWidget _aswbp_tutorial))
      (Class|CTutorialUI|SetAIPawn _output_get self)
      (bind _returnvalue (Actor|GetActorOfClass "/Game/LHJ/Tutorial/BP_TutorialManager.BP_TutorialManager_C"))
      (Variables|Default|SetTutorialManager _returnvalue)
      (CallFunction|SetWidgetVisible false))
    (:then_5
      ;[0.15 0.15 0.15 0.5] 발굴 맵 : 진행률UI, 시작 음성
      (bind _returnvalue_2 (Game|GetCurrentLevelName true))
      (if (Utilities|Enum|Equal(Enum) _returnvalue_2 "LV_TestExcavation")
        (bind _returnvalue_3 (Game|SpawnActorfromClass "/Game/LHM/BP/Excavation/BP_ProgressWidget.BP_ProgressWidget_C" (Math|Conversions|ToTransform(Vector) (Math|Vector|VectorZero)) "AlwaysSpawn" "MultiplyWithRoot" 0 0))
        (Transformation|AttachComponentToComponent _returnvalue_3 (Variables|Default|GetSkeletalMesh) "None" "KeepRelative" "KeepRelative" "KeepRelative" false)
        (CallFunction|PlayExcavationStart)))))

(event EventTick
  (params (DeltaSeconds :type Float%20%28single-precision%29))
  ;[0.15 0.15 0.15 0.5] Tick
  (Utilities|FlowControl|Sequence
    (:then_0
      (if (not (Variables|Default|GetbisLooking))
        (CallFunction|FollowtoLocation)))
    (:then_1
      (bind _asmh_vrplayer (Utilities|Casting|CastToMH_VRPlayer (Game|Player|GetPlayerPawn 0)))
      (Transformation|SetActorRotation (Math|Rotator|FindLookatRotation (Transformation|GetActorLocation) (Transformation|GetWorldLocation (Variables|/Script/GoGoHunters.MH_VRPlayer|GetVRCamera _asmh_vrplayer)))))))

(fn ConstructionScript)

(fn FollowtoLocation
  (bind _returnvalue (Transformation|GetActorLocation))
  (bind _returnvalue_2 (Transformation|GetActorLocation))
  (bind _movetolocation (Variables|Default|GetMoveToLocation))
  (bind _returnvalue_3 (Math|Rotator|FindLookatRotation _returnvalue_2 _movetolocation))
  (if (Variables|Default|GetbisFollowing)
    (if (Variables|Default|GetisMoveTo)
      (if (> (Math|Vector|VectorLength (- _returnvalue_2 _movetolocation)) (Variables|Default|GetMinMove))
        (Pawn|Input|AddMovementInput (Math|Vector|GetForwardVector (Math|Rotator|MakeRotator (.roll _returnvalue_3) (.pitch _returnvalue_3) (.yaw _returnvalue_3))) 1e+02 true))
      (else
        (bind _playershoulder (CallFunction|GetPlayerShoulderLocation))
        (if (> (Math|Vector|VectorLength (- _returnvalue _playershoulder)) (Variables|Default|GetMinMove))
          (Pawn|Input|AddMovementInput (Math|Vector|GetForwardVector (Math|Rotator|MakeRotator (.roll (Math|Rotator|FindLookatRotation _returnvalue _playershoulder)) (.pitch (Math|Rotator|FindLookatRotation _returnvalue _playershoulder)) (.yaw (Math|Rotator|FindLookatRotation _returnvalue _playershoulder)))) 1e+02 true))))))

(fn GetPlayerShoulderLocation
  (bind _attactpoint (Variables|Default|GetAttactPoint))
  (bind _asbp_mh_vrplayer (Utilities|Casting|CastToBP_MH_VRPlayer (Game|Player|GetPlayerPawn 0))
    (:then
      (Development|PrintString (Utilities|String|ToString(Vector) (.location (Transformation|GetBoneTransform (Variables|/Script/Engine.Character|GetMesh _asbp_mh_vrplayer) "root" "RTS_World"))))
      (return (+ (.location (Transformation|GetBoneTransform (Variables|/Script/Engine.Character|GetMesh _asbp_mh_vrplayer) "root" "RTS_World")) (* (Math|Vector|GetForwardVector (.rotation (Transformation|GetBoneTransform (Variables|/Script/Engine.Character|GetMesh _asbp_mh_vrplayer) "root" "RTS_World"))) (.x _attactpoint)) (* (Math|Vector|GetRightVector (.rotation (Transformation|GetBoneTransform (Variables|/Script/Engine.Character|GetMesh _asbp_mh_vrplayer) "root" "RTS_World"))) (.y _attactpoint)) (* (Math|Vector|GetUpVector (.rotation (Transformation|GetBoneTransform (Variables|/Script/Engine.Character|GetMesh _asbp_mh_vrplayer) "root" "RTS_World"))) (.z _attactpoint)))))
    (:CastFailed
      (return "0, 0, 0"))))

(fn LookingtoObject
  (if (Variables|Default|GetbisLooking)
    (bind _asabp_ai (Utilities|Casting|CastToABP_Ai (Components|SkeletalMesh|GetAnimInstance (Variables|Default|GetSkeletalMesh))))
    (Variables|/Game/Ai/Logic/ABP_Ai.ABP_Ai_C|SetLook%20At%20Location _asabp_ai (Transformation|GetActorLocation (Variables|Default|GetLookObject)))))

(fn SetTamiMesh
  (params (Enum :type E_Tami%20Enum :default "NewEnumerator0"))
  (Components|SkeletalMesh|SetSkeletalMeshAsset (Variables|Default|GetSkeletalMesh) (Utilities|Array|Get(acopy) (Variables|Default|GetSkeletalMeshAssetList) (Math|Conversions|ToInteger(Byte) (Utilities|Enum|LiteralenumE_Tami Enum)))))