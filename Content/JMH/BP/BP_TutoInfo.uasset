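; BP_TutoInfo is a tutorial info Blueprint that shows an egg restore guide through an animated widget.
; On BeginPlay it plays a timeline that moves the Move component vertically from its starting relative Z toward a fixed height.
; On each timeline update it also copies the guide text and texture into the WBP_EggRestoreGuide held by its Widget component.
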(event EventBeginPlay
  (bind _move (Variables|Default|Getmove))
  (Variables|Default|SetStartLoc (Variables|/Script/Engine.SceneComponent|GetRelativeLocation _move))
  (bind _newtrack_0 (Timeline|Timeline Play)
    (:Update
      (Transformation|SetRelativeLocation _move (Math|Vector|MakeVector (.x (Variables|Default|GetStartLoc)) (.y (Variables|Default|GetStartLoc)) (Math|Float|Lerp (.z (Variables|Default|GetStartLoc)) 1e+01 _newtrack_0)) false false)
      (bind _aswbp_egg_restore_guide (Utilities|Casting|CastToWBP_EggRestoreGuide (UserInterface|GetWidget (Variables|Default|GetWidget))))
      (Variables|/Game/JMH/UI/WBP_EggRestoreGuide.WBP_EggRestoreGuide_C|SetWBPText _aswbp_egg_restore_guide (Variables|Default|GetRestoreGuideText))
      (Variables|/Game/JMH/UI/WBP_EggRestoreGuide.WBP_EggRestoreGuide_C|SetWBPTexture _aswbp_egg_restore_guide (Variables|Default|GetWBPTexture)))))

(event Collision|EventActorBeginOverlap
  (params (OtherActor :type Actor%20Object%20Reference)))

(event EventTick
  (params (DeltaSeconds :type Float%20%28single-precision%29)))

(fn ConstructionScript)